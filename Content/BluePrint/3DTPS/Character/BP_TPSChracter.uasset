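; Third-person character Blueprint that wields a swappable weapon mesh and destroys whatever the weapon touches.
; BeginPlay starts a two-hand sword idle montage on the mesh, and Tick calls AnimationTick every frame.
; The 0 key steps WeaponIndex through WeaponArrays, wrapping to the start, and sets the selected static mesh on WeaponMesh.
; Any actor that begins overlapping WeaponMesh is destroyed immediately, with no filtering or damage step.
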(event `self.ReceiveBeginPlay`
  (`|PlayMontage` (`self.Mesh`) "/Game/Resources/Test/AnimationMesh/Montage/RPG-Character_2Hand-Sword-Idle_Montage.RPG-Character_2Hand-Sword-Idle_Montage"))

(event `self.ReceiveActorBeginOverlap`
  (params (OtherActor :type "Actor Object Reference")))

(event `self.ReceiveTick`
  (params (DeltaSeconds :type "Float (single-precision)"))
  (`self.AnimationTick`))

(event `Key|Zero`
  (params (Key :type "Key Structure"))
  (:`Pressed`
    (bind _result (`/Engine/EditorBlueprintResources/StandardMacros.IncrementInt` (`self.WeaponIndex`))
      (:`  `
        (if (>= _result (`KismetArrayLibrary.Array_Length` (`self.WeaponArrays`)))
          (set `self.WeaponIndex` 0))
        (`StaticMeshComponent.SetStaticMesh` (`self.WeaponMesh`) (`|GetArrayItem` (`self.WeaponArrays`) (`self.WeaponIndex`)))))))

(event `self.WeaponMesh.OnComponentBeginOverlap`
  (params (OverlappedComponent :type "PrimitiveComponent Object Reference") (OtherActor :type "Actor Object Reference") (OtherComp :type "PrimitiveComponent Object Reference") (OtherBodyIndex :type Integer) (bFromSweep :type Boolean) (SweepResult :type "HitResult Structure (by ref)"))
  (`self.K2_DestroyActor` OtherActor))

(fn `UserConstructionScript`)